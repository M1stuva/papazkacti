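; Game mode for an Old Maid card game between player characters and NPCs, running setup, turns and elimination.
; BeginPlay shuffles a deck built from the AllCards data table, deals it round-robin after a delay, removes pairs and starts play.
; A running counter modulo player count sets whose turn it is and advances on PlayerMoved.
; Empty-handed players are removed until the last is printed as loser; a separate check prints game end at any empty hand.
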(event `self.ReceiveBeginPlay`
  (`self.Make Deck`)
  (`KismetSystemLibrary.Delay` 2.0)
  (`self.Deal Cards`)
  (for _array_element (`self.Players`)
    (`/Game/Blueprints/Interfaces/BPI_Player.Remove Pairs` _array_element)
    (`self.abc` _array_element))
  (`self.Start Game`))

(event `Add Player`
  (params (Player :type "/Game/Blueprints/Interfaces/BPI_Player Interface"))
  (`KismetArrayLibrary.Array_AddUnique` (`self.Players`) Player))

(event `Remove Player`
  (params (Target :type "/Game/Blueprints/Interfaces/BPI_Player Interface"))
  (bind _players (`self.Players`))
  (bind _returnvalue (mod (`self.PlayerThatTakesCard`) (`KismetArrayLibrary.Array_Length` (`self.Players`))))
  (bind _returnvalue_2 (+ _returnvalue 0))
  (bind _length (`/Game/Blueprints/Interfaces/BPI_Player.Return Card List Length` Target))
  (if (== _length 0)
    (set `self.PlayerThatTakesCard` (select `bool` (== _returnvalue 0) :`false` _returnvalue_2 :`true` (+ _returnvalue_2 1)))
    (bind _asbp_npc (cast `/Game/Blueprints/Players/BP_NPC` Target)
      (:`then`
        (`/Game/Blueprints/Players/BP_NPC.Reset Card Actors` _asbp_npc))
      (:`CastFailed`
        (bind _asbp_old_maid_char (cast `/Game/Blueprints/Players/BP_OldMaidChar` Target)
          (:`then`
            (`/Game/Blueprints/Players/BP_OldMaidChar.Reset Card Actors` _asbp_old_maid_char))
          (:`CastFailed`
            _))))
    (`KismetArrayLibrary.Array_RemoveItem` _players Target)
    (if (== (`KismetArrayLibrary.Array_Length` _players) 1)
      (bind _asbp_npc_2 (cast `/Game/Blueprints/Players/BP_NPC` (`|GetArrayItem` _players))
        (:`then`
          (`KismetSystemLibrary.PrintString` (`KismetStringLibrary.Concat_StrStr` (`KismetSystemLibrary.GetDisplayName` _asbp_npc_2) " is loser") true true (struct :`R` 1.0 :`B` 0.924331 :`A` 1.0)))
        (:`CastFailed`
          (`KismetSystemLibrary.PrintString` "Player is loser" true true (struct :`R` 1.0 :`G` 0.012564 :`A` 1.0)))))))

(event `Start Game`
  (bind _players (`self.Players`))
  (for (_array_element _array_index) _players :!label _label
    (`/Game/Blueprints/Interfaces/BPI_Player.Set Player's Turn` _array_element (== _array_index (mod (`self.PlayerThatTakesCard`) (`KismetArrayLibrary.Array_Length` _players))))
    (`self.abc` _array_element)))

(event `Player Moved`
  (params (ItemToFind :type "/Game/Blueprints/Interfaces/BPI_Player Interface (by ref)"))
  (if (`KismetArrayLibrary.Array_Contains` (`self.Players`) ItemToFind)
    (`/Engine/EditorBlueprintResources/StandardMacros.IncrementInt` (`self.PlayerThatTakesCard`)
      (:`  `
        (goto _label)))))

(event `Check Is Game Finished`
  (for _array_element (`self.Players`)
    (bind _asbp_old_maid_char (cast `/Game/Blueprints/Players/BP_OldMaidChar` _array_element)
      (:`then`
        (if (== (`KismetArrayLibrary.Array_Length` (`/Game/Blueprints/Players/BP_OldMaidChar.Card List` _asbp_old_maid_char)) 0)
          (`|ExecutionSequence` :!label _label_2
            (:`then_0`
              (break))
            (:`then_1`
              (`KismetSystemLibrary.PrintString` "Game Ended" true true (struct :`R` 1.0 :`B` 0.272016 :`A` 1.0))))))
      (:`CastFailed`
        (bind _asbp_npc (cast `/Game/Blueprints/Players/BP_NPC` _array_element))
        (if (== (`KismetArrayLibrary.Array_Length` (`/Game/Blueprints/Players/BP_NPC.Card List` _asbp_npc)) 0)
          (goto _label_2))))))

(fn `abc`
  (params (Object :type "/Game/Blueprints/Interfaces/BPI_Player Interface"))
  (bind _asbp_npc (cast `/Game/Blueprints/Players/BP_NPC` Object)
    (:`then`
      (`KismetSystemLibrary.PrintString` (`KismetSystemLibrary.GetDisplayName` _asbp_npc) true true (struct :`G` 0.66 :`B` 1.0 :`A` 1.0) 15.0))
    (:`CastFailed`
      (bind _asbp_old_maid_char (cast `/Game/Blueprints/Players/BP_OldMaidChar` Object))
      (`KismetSystemLibrary.PrintString` (`KismetSystemLibrary.GetDisplayName` _asbp_old_maid_char) true true (struct :`G` 0.66 :`B` 1.0 :`A` 1.0) 15.0))))

(fn `Deal Cards`
  (bind _card_list (`self.Card List`))
  (for (_array_element _array_index) _card_list
    (`/Game/Blueprints/Interfaces/BPI_Player.Get Card` (`|GetArrayItem` (`self.Players`) (mod _array_index (`KismetArrayLibrary.Array_Length` (`self.Players`)))) _array_element))
  (set `self.PlayerThatTakesCard` (`KismetArrayLibrary.Array_Length` _card_list)))

(fn `Make Deck`
  (bind _outrownames (`DataTableFunctionLibrary.GetDataTableRowNames` "/Game/Blueprints/DataTables/AllCards.AllCards"))
  (for _array_element _outrownames
    (bind _returnvalue (`|GetDataTableRow` "/Game/Blueprints/DataTables/AllCards.AllCards" _array_element)
      (:`then`
        (`KismetArrayLibrary.Array_Add` (`self.Card List`) _returnvalue))))
  (`KismetArrayLibrary.Array_Shuffle` (`self.Card List`))
  (return))

(fn `UserConstructionScript`)