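; BP_Card is an interactable playing card actor whose mesh comes from its CardValue data.
; The construction script applies that card model to the static mesh.
; On BeginPlay, it destroys its ChildActor component if the owning player is a BP_OldMaidChar.
; Interface focus toggles custom depth rendering on the mesh, while the interact event and widget getter are empty stubs.
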(event `self.ReceiveBeginPlay`
  (cast `/Game/Blueprints/Players/BP_OldMaidChar` (`self.OwnerPlayer`))
  (`ActorComponent.K2_DestroyComponent` (`self.ChildActor`)))

(event `/Game/Interaction/BPI_Interaction.Interface_ToggleFocus`
  (params (Focus :type Boolean))
  (`PrimitiveComponent.SetRenderCustomDepth` (`self.StaticMesh`) Focus))

(event `/Game/Interaction/BPI_Interaction.InterfaceInteract`)

(fn `GetInteractionWidgetRef`
  (returns (Ref :type "WidgetComponent Object Reference"))
  (return null))

(fn `UserConstructionScript`
  (bind (_card_value_cardvalue _card_value_cardskin _card_value_cardmodel) (break `/Game/Blueprints/Structures/S_Card` (`self.Card Value`)))
  (`StaticMeshComponent.SetStaticMesh` (`self.StaticMesh`) _card_value_cardmodel))