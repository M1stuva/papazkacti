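; AI opponent for the Old Maid card game that registers with BP_OldMaid_GameMode at BeginPlay.
; On its turn it waits a random delay, draws a random card from the preceding player, then reports to the game mode.
; Each hand change recursively discards pairs and respawns BP_Card actors in a fan.
; Die slides the mesh along local Y with a timeline, then destroys the actor.
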(event `self.ReceiveBeginPlay`
  (`KismetSystemLibrary.Delay` 0.0)
  (bind _asbp_old_maid_game_mode (cast `/Game/Blueprints/GameMode/BP_OldMaid_GameMode` (`GameplayStatics.GetGameMode`)))
  (bind _output_get (set `self.GameMode` _asbp_old_maid_game_mode))
  (`/Game/Blueprints/GameMode/BP_OldMaid_GameMode.Add Player` _output_get self))

(event `self.Remove Pairs`
  (bind (_returnvalue_roll _returnvalue_pitch _returnvalue_yaw) (`KismetMathLibrary.BreakRotator` (`self.K2_GetActorRotation`)))
  ;[0.1562 0.1562 0.1562] Kartları elden çıkarıp elde oluşmasını sağlar
  (`self.Remove Pairs Func`)
  (for (_array_element _array_index) (`self.Card List`)
    (bind _returnvalue (`|SpawnActorFromClass` "/Game/Blueprints/GameObjects/BP_Card.BP_Card_C" (`KismetMathLibrary.MakeTransform` (+ (`SceneComponent.K2_GetComponentLocation` (`self.Card Spawn Point`)) (* (+ (* (`self.GetActorRightVector`) 3.0) (* (`self.GetActorForwardVector`) -0.5) (0.0 0.0 0.02)) _array_index)) (`KismetMathLibrary.MakeRotator` _returnvalue_roll (* -10.0 _array_index) (+ _returnvalue_yaw 180.0))) "Undefined" "MultiplyWithRoot" null _array_element self null))
    (`KismetArrayLibrary.Array_Add` (`self.CardActors`) _returnvalue)))

(event `self.Get Card`
  (params (Card :type "/Game/Blueprints/Structures/S_Card Structure"))
  (`KismetArrayLibrary.Array_Add` (`self.Card List`) Card))

(event `self.Set Player's Turn`
  (params (`Is Player's Turn` :type Boolean))
  (bind _gamemode (`self.GameMode`))
  (bind _output (`|GetArrayItem` (`/Game/Blueprints/GameMode/BP_OldMaid_GameMode.Players` _gamemode) (mod (- (`/Game/Blueprints/GameMode/BP_OldMaid_GameMode.PlayerThatTakesCard` _gamemode) 1) (`KismetArrayLibrary.Array_Length` (`/Game/Blueprints/GameMode/BP_OldMaid_GameMode.Players` _gamemode)))))
  ;[0.2708 0.2708 0.2708] NPC kendi turuysa hamlesini yapıyor
  (bind _output_get (set `self.Is Player's Turn` `Is Player's Turn`))
  (if _output_get
    (`KismetSystemLibrary.Delay` (`KismetMathLibrary.RandomFloatInRange` 0.5 3.0))
    (bind _length (`self.Return Card List Length` _output))
    (`self.Give Card` _output (`KismetMathLibrary.RandomIntegerInRange` 0 (- _length 1)) self)
    (`self.Reset Card Actors`)
    (`/Game/Blueprints/GameMode/BP_OldMaid_GameMode.Remove Player` (`self.GameMode`) self)
    (`KismetSystemLibrary.Delay` 0.2)
    (`/Game/Blueprints/GameMode/BP_OldMaid_GameMode.Player Moved` (`self.GameMode`) self)))

(event `self.Give Card`
  (params (`Card Index` :type Integer) (Player :type "/Game/Blueprints/Interfaces/BPI_Player Interface"))
  (bind _card_list (`self.Card List`))
  (`self.Get Card` Player (`|GetArrayItem` _card_list `Card Index`))
  (`KismetArrayLibrary.Array_Remove` _card_list `Card Index`)
  (`self.Reset Card Actors`)
  (`/Game/Blueprints/GameMode/BP_OldMaid_GameMode.Remove Player` (`self.GameMode`) self))

(event `Reset Card Actors`
  (bind _cardactors (`self.CardActors`))
  (for _array_element _cardactors
    (`/Engine/EditorBlueprintResources/StandardMacros.IsValid` _array_element
      (:`Is Valid`
        (`self.K2_DestroyActor` _array_element))))
  (`KismetArrayLibrary.Array_Clear` _cardactors)
  (`self.Remove Pairs`))

(event `Die`
  (bind (_direction _lerp) (`Timeline|Timeline`)
    (:`Update`
      (`SceneComponent.K2_SetRelativeLocation` (`self.SkeletalMesh`) (`KismetMathLibrary.MakeVector` 0.0 (`KismetMathLibrary.Lerp` 0.0 -250.0 _lerp)) false false))
    (:`Finished`
      (`self.K2_DestroyActor`))))

(fn `Remove Pairs Func`
  (bind _card_list (`self.Card List`))
  (for (_array_element _array_index) _card_list :!label _label
    (for _index (range (+ _array_index 1) (`KismetArrayLibrary.Array_Length` _card_list))
      (bind _output (`|GetArrayItem` (`self.Card List`) _index))
      (if (`|EnumEquality` (`.CardValue_3_140664B74346FFCFD46A52A5253F676D` (break `/Game/Blueprints/Structures/S_Card` _output)) (`.CardValue_3_140664B74346FFCFD46A52A5253F676D` (break `/Game/Blueprints/Structures/S_Card` _array_element)))
        (`KismetArrayLibrary.Array_RemoveItem` (`self.Card List`) _output)
        (`KismetArrayLibrary.Array_RemoveItem` (`self.Card List`) _array_element)
        (`|ExecutionSequence`
          (:`then_0`
            (break))
          (:`then_1`
            (goto _label :!via `Break`))
          (:`then_2`
            (`self.Remove Pairs Func`)))))))

(fn `Return Card List Length`
  (returns (Length :type Integer))
  (return (`KismetArrayLibrary.Array_Length` (`self.Card List`))))

(fn `UserConstructionScript`)